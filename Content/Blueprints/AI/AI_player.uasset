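; AI-controlled player pawn that faces its direction of movement and fires cannonballs from a limited ammo count.
; RotationAngle derives yaw from velocity using per-quadrant arctangent math, and Update Animation applies it as control rotation.
; Shooting spawns a CanonBall below the actor along that yaw while Armo remains, then decrements the count, which Get_Armo exposes.
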(fn `Get_Armo`
  (returns (Armo :type Integer))
  (return (`self.Armo`)))

(fn `RotationAngle`
  (params (NewParam :type "Rotator Structure"))
  (returns (ReturnValue :type "Rotator Structure"))
  (bind (_returnvalue_x _returnvalue_y) (`KismetMathLibrary.BreakVector` (`self.GetVelocity`)))
  (bind (_returnvalue_x_2 _returnvalue_y_2) (`KismetMathLibrary.BreakVector` (`self.GetVelocity`)))
  (bind (_returnvalue_x_3 _returnvalue_y_3) (`KismetMathLibrary.BreakVector` (`self.GetVelocity`)))
  (bind (_returnvalue_x_4 _returnvalue_y_4) (`KismetMathLibrary.BreakVector` (`self.GetVelocity`)))
  (bind (_returnvalue_x_5 _returnvalue_y_5) (`KismetMathLibrary.BreakVector` (`self.GetVelocity`)))
  (bind _returnvalue (> _returnvalue_y_2 0.0))
  (if (> _returnvalue_x_2 0.0)
    (if _returnvalue
      (return (`KismetMathLibrary.MakeRotator` 0.0 0.0 (`KismetMathLibrary.DegAtan` (/ _returnvalue_y_3 _returnvalue_x_3))))
      (else
        (return (`KismetMathLibrary.MakeRotator` 0.0 0.0 (- 360.0 (`KismetMathLibrary.DegAtan` (/ (* _returnvalue_y_4 -1.0) _returnvalue_x_4)))))))
    (elif _returnvalue
      (return (`KismetMathLibrary.MakeRotator` 0.0 0.0 (- 180.0 (`KismetMathLibrary.DegAtan` (/ _returnvalue_y (* _returnvalue_x -1.0))))))
      (else
        (return (`KismetMathLibrary.MakeRotator` 0.0 0.0 (+ 180.0 (`KismetMathLibrary.DegAtan` (/ (* _returnvalue_y_5 -1.0) (* _returnvalue_x_5 -1.0))))))))))

(fn `Shooting`
  (if (> (`self.Armo`) 0)
    (bind _returnvalue (`self.RotationAngle` (struct)))
    (`|SpawnActorFromClass` "/Game/Blueprints/CanonBall.CanonBall_C" (`KismetMathLibrary.MakeTransform` (`KismetMathLibrary.MakeVector` (.x (`self.K2_GetActorLocation`)) (.y (`self.K2_GetActorLocation`)) (- (.z (`self.K2_GetActorLocation`)) 70.0)) _returnvalue) "AlwaysSpawn" "MultiplyWithRoot" null null)
    (bind _result (`/Engine/EditorBlueprintResources/StandardMacros.DecrementInt` (`self.Armo`))
      (:`  `
        (set `self.Armo` _result)))))

(fn `Update Animation`
  (bind _returnvalue (`self.RotationAngle` (struct)))
  (`Controller.SetControlRotation` (`self.GetController`) _returnvalue))

(fn `UserConstructionScript`)